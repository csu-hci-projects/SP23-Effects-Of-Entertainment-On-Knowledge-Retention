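; BP_TowerActor is a tower defense turret that automatically turns toward and shoots at enemies.
; AddEnemyFunc adds enemies to EnemyList, and EndActorOverlap removes them when they leave.
; Each Tick, the tower smoothly yaws toward the first listed enemy and, when CanFire allows, spawns a BP_Bullet2 aimed at that enemy's LeadingTarget.
; It draws a debug trace per shot, then resets CanFire after a FireRate-based delay.
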(event Collision|EventActorEndOverlap
  (params (OtherActor :type Actor%20Object%20Reference))
  ;[1 1 1] Remove Enemy from array after they have gone too far away
  (bind _asbp_enemy_character (Utilities|Casting|CastToBP_enemy_character OtherActor))
  (Utilities|Array|RemoveItem (Variables|Default|GetEnemyList) _asbp_enemy_character))

(event EventTick
  (params (DeltaSeconds :type Float%20%28single-precision%29))
  (bind _self self)
  (bind _enemylist (Variables|Default|GetEnemyList))
  (bind _enemylist_2 (Variables|Default|GetEnemyList))
  (bind _output (Utilities|Array|Get(acopy) _enemylist_2))
  (bind _output_2 (Utilities|Array|Get(acopy) _enemylist))
  ;[1 1 1] Every Tick, if there is an enemy in the array, then...
  (if (Utilities|Array|IsValidIndex _enemylist)
    (if (Utilities|IsValid _output_2)
      ;[1 1 1] First, Rotate to point at the enemy
      (Utilities|FlowControl|Sequence
        (:then_0
          (Transformation|SetActorRotation (Math|Interpolation|RInterpTo (Transformation|GetActorRotation _self) (Math|Rotator|MakeRotator 0.0 0.0 (.yaw (Math|Rotator|FindLookatRotation (Transformation|GetActorLocation _self) (Transformation|GetActorLocation _output_2)))) (Utilities|Time|GetWorldDeltaSeconds) 1e+01)))
        (:then_1
          ;[1 1 1] Second, fire a bullet
          (if (Variables|Default|GetCanFire?)
            (bind _returnvalue (Game|SpawnActorfromClass "/Game/Tower_Defense/BP_Bullet2.BP_Bullet2_C" (Transformation|GetWorldTransform (Variables|Default|GetArrow)) "AlwaysSpawn" 0 0))
            (Variables|/Game/Tower_Defense/BP_Bullet2.BP_Bullet2_C|SetTargetLocation _returnvalue (Transformation|GetWorldTransform (Variables|/Game/Tower_Defense/BP_enemy_character.BP_enemy_character_C|GetLeading%20Target _output)))
            (Collision|LineTraceByChannel (Transformation|GetWorldLocation (Variables|Default|GetArrow)) (Transformation|GetWorldLocation (Variables|/Game/Tower_Defense/BP_enemy_character.BP_enemy_character_C|GetChest _output)) "TraceTypeQuery1" false 0 "ForDuration" true "(R=1.000000,G=0.000000,B=0.000000,A=1.000000)" "(R=1.000000,G=0.000000,B=0.000000,A=1.000000)" 0.1)
            (Variables|Default|SetCanFire? false)
            (Utilities|FlowControl|Delay 0.1)
            (Utilities|FlowControl|Delay (Variables|Default|GetFireRate))
            (Variables|Default|SetCanFire? true)))))))

(fn ConstructionScript)

(fn AddEnemyFunc
  (params (Enemy%20Ref :type BP%20Enemy%20Character%20Object%20Reference))
  (Utilities|Array|AddUnique (Variables|Default|GetEnemyList) Enemy%20Ref))