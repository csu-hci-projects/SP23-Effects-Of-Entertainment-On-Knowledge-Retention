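; Tower defense spawner that releases a wave of enemy characters, then opens a question-and-answer screen once none remain.
; From BeginPlay, a delayed loop spawns AI at the sphere component's location until the enemy count runs out.
; Each enemy joins EnemyList and takes the remaining count as its threat order.
; After the last spawn, it polls for surviving enemies and adds the widget to the viewport when all are gone.
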(event Custom|SpawnEnemy
  (bind _returnvalue (AI|SpawnAIFromClass "/Game/Tower_Defense/BP_enemy_character.BP_enemy_character_C" 0 (Transformation|GetWorldLocation (Variables|Default|GetSphewre)) "0, 0, 0" false 0))
  (bind _asbp_enemy_character (Utilities|Casting|CastToBP_enemy_character _returnvalue))
  (Variables|/Game/Tower_Defense/BP_enemy_character.BP_enemy_character_C|SetVolume%28Threat/order%29 _asbp_enemy_character (Variables|Default|GetNumEnemies))
  (Utilities|Array|Add (Variables|Default|GetEnemyList) _asbp_enemy_character))

(event EventBeginPlay
  (Utilities|FlowControl|Delay (Variables|Default|GetSpawnRate) :!label _label)
  (CallFunction|SpawnEnemy)
  (bind _result (Math|Integer|DecrementInt (Variables|Default|GetNumEnemies))
    (:%20%20
      (if (<= _result 0)
        (bind _outactors (Actor|GetAllActorsOfClass "/Game/Tower_Defense/BP_enemy_character.BP_enemy_character_C" :!label _label_2))
        (if (Utilities|Array|IsEmpty _outactors)
          (bind _returnvalue (UserInterface|CreateWidget "/Game/Tower_Defense/QuestionNAnswer_Widget.QuestionNAnswer_Widget_C"))
          (UserInterface|Viewport|AddtoViewport _returnvalue 0)
          (else
            (Utilities|FlowControl|Delay 2.0)
            (goto _label_2)))
        (else
          (goto _label))))))

(fn ConstructionScript)