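; BP_enemy_character is a tower defense enemy that walks toward the level's target point and can be shot by towers.
; Shortly after spawning it uses AI Move To toward the first TargetPoint found, destroying itself on arrival.
; Overlapping a BP_TowerActor registers the enemy with that tower through AddEnemyFunc.
; Its GetShot event destroys it immediately, with no health check.
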(event Custom|GetShot
  ;[1 1 1] Destory self when shot
  (Actor|DestroyActor))

(event EventBeginPlay
  ;[1 1 1] Move to target after spawning
  (Utilities|FlowControl|Delay 0.001)
  (bind _returnvalue (Actor|GetActorOfClass "/Script/Engine.TargetPoint"))
  (AI|AIMoveTo self (Transformation|GetActorLocation _returnvalue) 0 5.0 true
    (:OnSuccess
      (Actor|DestroyActor))))

(event Collision|EventActorBeginOverlap
  (params (OtherActor :type Actor%20Object%20Reference))
  ;[1 1 1] Add self to the array of enemies inside the tower it just touched
  (bind _asbp_tower_actor (Utilities|Casting|CastToBP_TowerActor OtherActor))
  (Default|AddEnemyFunc _asbp_tower_actor self))

(fn ConstructionScript)